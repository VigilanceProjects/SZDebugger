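; BP_DebugArrow is a short-lived debug actor that displays an arrow pointing along a given vector.
; On BeginPlay it orients its Arrow component and applies the configured color, size and length, then destroys itself after Duration.
; The delay is multiplied by global time dilation so lifetime follows real time, and a zero or negative Duration keeps the arrow only until the next tick.
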(event `self.ReceiveBeginPlay`
  (bind _duration (`self.Duration`))
  (bind _arrow (`self.Arrow`))
  (`SceneComponent.K2_SetWorldRotation` (`self.Arrow`) (`KismetMathLibrary.Conv_VectorToRotator` (`self.Vector`)) false false)
  (`ArrowComponent.SetArrowColor` (`self.Arrow`) (`self.Color`))
  (set `ArrowComponent.ArrowSize` (`self.ArrowSize`) _arrow)
  (set `ArrowComponent.ArrowLength` (`self.ArrowLength`) _arrow)
  (if (<= _duration 0.0)
    (`KismetSystemLibrary.DelayUntilNextTick`)
    (else
      (`KismetSystemLibrary.Delay` (* _duration (`GameplayStatics.GetGlobalTimeDilation`)))))
  (`self.K2_DestroyActor`))

(fn `UserConstructionScript`)