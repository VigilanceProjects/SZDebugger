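; Free-flying debug camera pawn with Enhanced Input movement, speed modifiers, look, roll, FOV control and toggleable spring-arm lag.
; Movement offsets the actor without sweeping, and setters can lock moving or looking.
; Mouse-ray traces from the camera feed hover, click and release dispatchers for listeners, with hover hitting only Vehicle objects.
; While possessed, Tick throttles hover traces with a Delay, skipped under heavy slow motion; unpossessing also notifies listeners.
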(event `self.ReceivePossessed`
  (params (NewController :type "Controller Object Reference"))
  (set `self.TraceHover` true))

(event `self.ReceiveUnpossessed`
  (params (OldController :type "Controller Object Reference"))
  (`self.OnUnpossessed`)
  (set `self.TraceHover` false))

(event `self.ReceiveBeginPlay`
  (`EnhancedInputSubsystemInterface.AddMappingContext` (pcsubsystem `EnhancedInputLocalPlayerSubsystem` (`GameplayStatics.GetPlayerController` 0)) "/SZDebugger/BP/Input/DebugPawn/IMC_DebugPawn.IMC_DebugPawn" 5 (struct)))

(event `EnhancedInput|/SZDebugger/BP/Input/DebugPawn/IA_ChangeFOV`
  (params (ActionValue :type "Float (double-precision)") (ElapsedSeconds :type "Float (double-precision)") (TriggeredSeconds :type "Float (double-precision)") (InputAction :type "InputAction Object Reference" :default "/SZDebugger/BP/Input/DebugPawn/IA_ChangeFOV.IA_ChangeFOV"))
  (bind _camera (`self.Camera`))
  (:`Triggered`
    (`CameraComponent.SetFieldOfView` _camera (`KismetMathLibrary.FClamp` (+ (`CameraComponent.FieldOfView` _camera) (* ActionValue 3.0)) 1.0 155.0))))

(event `EnhancedInput|/SZDebugger/BP/Input/DebugPawn/IA_Look`
  (params (ActionValue :type "Vector2D Structure") (ElapsedSeconds :type "Float (double-precision)") (TriggeredSeconds :type "Float (double-precision)") (InputAction :type "InputAction Object Reference" :default "/SZDebugger/BP/Input/DebugPawn/IA_Look.IA_Look"))
  (:`Triggered`
    (set `self.MouseValue` (`KismetMathLibrary.MakeVector2D` ActionValue_X ActionValue_Y))
    (if (`self.CanLookAround`)
      (`self.AddControllerPitchInput` ActionValue_X)
      (`self.AddControllerYawInput` ActionValue_Y)))
  (:`Canceled`
    (set `self.MouseValue` (0.0 0.0) :!label _label))
  (:`Completed`
    (goto _label)))

(event `EnhancedInput|/SZDebugger/BP/Input/DebugPawn/IA_MoveVertically`
  (params (ActionValue :type "Float (double-precision)") (ElapsedSeconds :type "Float (double-precision)") (TriggeredSeconds :type "Float (double-precision)") (InputAction :type "InputAction Object Reference" :default "/SZDebugger/BP/Input/DebugPawn/IA_MoveVertically.IA_MoveVertically"))
  (:`Triggered`
    (if (`self.CanMove`)
      (`self.K2_SetActorLocation` (+ (`self.K2_GetActorLocation`) (`KismetMathLibrary.MakeVector` 0.0 0.0 (* (`self.MovementSpeed`) (`self.SpeedMultiplier`) ActionValue)))))))

(event `EnhancedInput|/SZDebugger/BP/Input/DebugPawn/IA_Move`
  (params (ActionValue :type "Vector2D Structure") (ElapsedSeconds :type "Float (double-precision)") (TriggeredSeconds :type "Float (double-precision)") (InputAction :type "InputAction Object Reference" :default "/SZDebugger/BP/Input/DebugPawn/IA_Move.IA_Move"))
  (:`Triggered`
    (if (`self.CanMove`)
      (`self.UpdatePawnLocationFromMoveIA` ActionValue))))

(event `EnhancedInput|/SZDebugger/BP/Input/IA_LeftShift`
  (params (ActionValue :type Boolean) (ElapsedSeconds :type "Float (double-precision)") (TriggeredSeconds :type "Float (double-precision)") (InputAction :type "InputAction Object Reference" :default "/SZDebugger/BP/Input/IA_LeftShift.IA_LeftShift"))
  (:`Started`
    (set `self.MovementSpeed` (* (`self.DEFAULT_MOVEMENT_SPEED`) 4.0)))
  (:`Canceled`
    (set `self.MovementSpeed` (`self.DEFAULT_MOVEMENT_SPEED`) :!label _label_2))
  (:`Completed`
    (goto _label_2)))

(event `EnhancedInput|/SZDebugger/BP/Input/IA_LeftCtrl`
  (params (ActionValue :type Boolean) (ElapsedSeconds :type "Float (double-precision)") (TriggeredSeconds :type "Float (double-precision)") (InputAction :type "InputAction Object Reference" :default "/SZDebugger/BP/Input/IA_LeftCtrl.IA_LeftCtrl"))
  (:`Started`
    (set `self.MovementSpeed` (/ (`self.DEFAULT_MOVEMENT_SPEED`) 3.0)))
  (:`Canceled`
    (set `self.MovementSpeed` (`self.DEFAULT_MOVEMENT_SPEED`) :!label _label_3))
  (:`Completed`
    (goto _label_3)))

(event `EnhancedInput|/SZDebugger/BP/Input/DebugPawn/IA_ChangeRoll`
  (params (ActionValue :type "Float (double-precision)") (ElapsedSeconds :type "Float (double-precision)") (TriggeredSeconds :type "Float (double-precision)") (InputAction :type "InputAction Object Reference" :default "/SZDebugger/BP/Input/DebugPawn/IA_ChangeRoll.IA_ChangeRoll"))
  (:`Triggered`
    (if (`self.CanLookAround`)
      (`self.AddControllerRollInput` ActionValue))))

(event `EnhancedInput|/SZDebugger/BP/Input/DebugPawn/IA_ResetRoll`
  (params (ActionValue :type Boolean) (ElapsedSeconds :type "Float (double-precision)") (TriggeredSeconds :type "Float (double-precision)") (InputAction :type "InputAction Object Reference" :default "/SZDebugger/BP/Input/DebugPawn/IA_ResetRoll.IA_ResetRoll"))
  (bind _returnvalue (`GameplayStatics.GetPlayerController` 0))
  (bind (_returnvalue_roll _returnvalue_pitch _returnvalue_yaw) (`KismetMathLibrary.BreakRotator` (`Controller.GetControlRotation` _returnvalue)))
  (:`Started`
    (if (`self.CanLookAround`)
      (`Controller.SetControlRotation` _returnvalue (`KismetMathLibrary.MakeRotator` 0.0 _returnvalue_pitch _returnvalue_yaw)))))

(event `EnhancedInput|/SZDebugger/BP/Input/DebugPawn/IA_ChangeMoveSpeedMultiplier`
  (params (ActionValue :type "Float (double-precision)") (ElapsedSeconds :type "Float (double-precision)") (TriggeredSeconds :type "Float (double-precision)") (InputAction :type "InputAction Object Reference" :default "/SZDebugger/BP/Input/DebugPawn/IA_ChangeMoveSpeedMultiplier.IA_ChangeMoveSpeedMultiplier"))
  (:`Triggered`
    (set `self.SpeedMultiplier` (`KismetMathLibrary.FClamp` (+ (`self.SpeedMultiplier`) (/ ActionValue 10.0)) 0.1 5.0))))

(event `EnhancedInput|/SZDebugger/BP/Input/DebugPawn/IA_TraceMouseClick`
  (params (ActionValue :type "Vector2D Structure") (ElapsedSeconds :type "Float (double-precision)") (TriggeredSeconds :type "Float (double-precision)") (InputAction :type "InputAction Object Reference" :default "/SZDebugger/BP/Input/DebugPawn/IA_TraceMouseClick.IA_TraceMouseClick"))
  (:`Started`
    (bind _outhit (`self.TraceMouseClick`))
    (`self.OnMouseClick` _outhit))
  (:`Canceled`
    (`self.OnMouseRelease` :!label _label_4))
  (:`Completed`
    (goto _label_4)))

(event `EnhancedInput|/SZDebugger/BP/Input/DebugPawn/IA_SwitchSmoothCamMode`
  (params (ActionValue :type "Vector2D Structure") (ElapsedSeconds :type "Float (double-precision)") (TriggeredSeconds :type "Float (double-precision)") (InputAction :type "InputAction Object Reference" :default "/SZDebugger/BP/Input/DebugPawn/IA_SwitchSmoothCamMode.IA_SwitchSmoothCamMode"))
  (:`Started`
    (`self.SetCameraLagEnabled` (not (`self.CameraLagEnabled`)))))

(event `self.ReceiveTick`
  (params (DeltaSeconds :type "Float (single-precision)"))
  (if (`self.TraceHover`)
    (if (not (< (`GameplayStatics.GetGlobalTimeDilation`) 0.3))
      (`KismetSystemLibrary.Delay` 0.1))
    (`self.HandleCallOnMouseHover`)))

(fn `HandleCallOnMouseHover`
  (bind _outhit (`self.TraceMouseHover`))
  (`self.OnMouseHover` _outhit))

(fn `SetCameraLagEnabled`
  (params (Enabled :type Boolean))
  (bind _springarm (`self.SpringArm`))
  (set `self.CameraLagEnabled` Enabled)
  (set `SpringArmComponent.bEnableCameraLag` Enabled _springarm)
  (set `SpringArmComponent.bEnableCameraRotationLag` Enabled _springarm))

(fn `SetCanLookAround`
  (params (CanLookAround :type Boolean))
  (set `self.CanLookAround` CanLookAround))

(fn `SetCanMove`
  (params (CanMove :type Boolean))
  (set `self.CanMove` CanMove))

(fn `TraceMouseClick`
  (returns (OutHit :type "HitResult Structure") (ReturnValue :type Boolean))
  (bind _returnvalue (`SceneComponent.K2_GetComponentLocation` (`self.Camera`)))
  (bind (_outhit _returnvalue_2) (`KismetSystemLibrary.LineTraceSingleForObjects` :`Start` _returnvalue :`End` (+ _returnvalue (* (`.WorldDirection` (`PlayerController.DeprojectMousePositionToWorld` (`GameplayStatics.GetPlayerController` 0))) 1000000.0)) :`ObjectTypes` (`|MakeArray` "ObjectTypeQuery1" "ObjectTypeQuery13" "ObjectTypeQuery14" "ObjectTypeQuery15" "ObjectTypeQuery16" "ObjectTypeQuery17" "ObjectTypeQuery18" "ObjectTypeQuery5" "ObjectTypeQuery6" "ObjectTypeQuery10" "ObjectTypeQuery12" "ObjectTypeQuery3" "ObjectTypeQuery9" "ObjectTypeQuery8" :!type "EObjectTypeQuery Enum") :`bTraceComplex` true :`DrawDebugType` "ForDuration"))
  (return _outhit _returnvalue_2))

(fn `TraceMouseHover`
  (returns (OutHit :type "HitResult Structure") (ReturnValue :type Boolean))
  (bind _returnvalue (`SceneComponent.K2_GetComponentLocation` (`self.Camera`)))
  (bind (_outhit _returnvalue_2) (`KismetSystemLibrary.LineTraceSingleForObjects` _returnvalue (+ _returnvalue (* (`.WorldDirection` (`PlayerController.DeprojectMousePositionToWorld` (`GameplayStatics.GetPlayerController` 0))) 10000000.0)) (`|MakeArray` "ObjectTypeQuery5" :!type "EObjectTypeQuery Enum") true))
  (return _outhit _returnvalue_2))

(fn `UpdatePawnLocationFromMoveIA`
  (params (ActionValue :type "Vector2D Structure"))
  (bind _returnvalue (* (`self.MovementSpeed`) (`self.SpeedMultiplier`)))
  (`self.K2_SetActorLocation` (+ (+ (`self.K2_GetActorLocation`) (* (`self.GetActorForwardVector`) (* ActionValue_X _returnvalue))) (* (`self.GetActorRightVector`) (* ActionValue_Y _returnvalue)))))

(fn `UserConstructionScript`)