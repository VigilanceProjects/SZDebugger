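; Preview renderer Blueprint that captures isolated images of static or skeletal meshes with given materials through a SceneCaptureComponent2D.
; Entry functions assign the mesh and materials to their component, then trigger a capture after a delay scaled by global time dilation.
; Capture uses component bounds to set spotlight intensity, offset the camera diagonally and aim it at the bounds origin, then renders only that component via the show-only list.
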(event `CE_Capture`
  (params (PrimitiveComponentToCapture :type "PrimitiveComponent Object Reference") (DelayBeforeCapture :type "Float (double-precision)"))
  (`KismetSystemLibrary.Delay` (* DelayBeforeCapture (`GameplayStatics.GetGlobalTimeDilation`)))
  (`self.Capture` PrimitiveComponentToCapture))

(fn `Capture`
  (params (PrimitiveComponentToCapture :type "PrimitiveComponent Object Reference"))
  (bind _scenecapturecomponent2d (`self.SceneCaptureComponent2D`))
  (bind (_origin _boxextent _sphereradius) (`KismetSystemLibrary.GetComponentBounds` (`local.PrimitiveComponentToCapture`)))
  (`LightComponent.SetIntensity` (`self.SpotLight`) (`KismetMathLibrary.FClamp` (* _sphereradius 75.0) 0.0 500000.0))
  (`SceneComponent.K2_SetRelativeLocation` (`self.SceneCaptureComponent2D`) (+ _boxextent (* (`KismetMathLibrary.VSize` _boxextent) 0.3)) false false)
  (`SceneComponent.K2_SetRelativeRotation` (`self.SceneCaptureComponent2D`) (`KismetMathLibrary.FindLookAtRotation` (`SceneComponent.K2_GetComponentLocation` (`self.SceneCaptureComponent2D`)) _origin) false false)
  (`SceneCaptureComponent.ClearShowOnlyComponents` _scenecapturecomponent2d)
  (`SceneCaptureComponent.ShowOnlyComponent` _scenecapturecomponent2d (`local.PrimitiveComponentToCapture`))
  (`SceneCaptureComponent2D.CaptureScene` (`self.SceneCaptureComponent2D`)))

(fn `CaptureSkeletalMesh`
  (params (SKLMesh :type "SkeletalMesh Object Reference") (UsedMats :type "Array of MaterialInterface Object Reference") (DelayBeforeCapture :type "Float (double-precision)" :default 0.1))
  (bind _skeletalmesh (`self.SkeletalMesh`))
  (`SkeletalMeshComponent.SetSkeletalMeshAsset` _skeletalmesh SKLMesh)
  (`/SZDebugger/BP/BPFL/BPFL_PrimitiveComponentUtility.SetMaterials` _skeletalmesh UsedMats)
  (`self.CE_Capture` _skeletalmesh DelayBeforeCapture))

(fn `CaptureStaticMesh`
  (params (StaticMesh :type "StaticMesh Object Reference") (UsedMats :type "Array of MaterialInterface Object Reference") (DelayBeforeCapture :type "Float (double-precision)" :default 0.1))
  (bind _staticmesh (`self.StaticMesh`))
  (`StaticMeshComponent.SetStaticMesh` _staticmesh StaticMesh)
  (`/SZDebugger/BP/BPFL/BPFL_PrimitiveComponentUtility.SetMaterials` _staticmesh UsedMats)
  (`self.CE_Capture` _staticmesh DelayBeforeCapture))

(fn `UserConstructionScript`)