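; BP_3DAxes is a 3D transform gizmo with X, Y, Z and All handles for location, rotation or scale.
; Hover events drive axis selection, swapping the handle's material to a highlight unless the selection is locked.
; SetAxesType swaps handle meshes and orientations and hides All for rotation.
; It exposes the selected axis's world vector from the mesh's forward vector, with absolute scale and optional absolute rotation set on the parent component.
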(event `self.ReceiveBeginPlay`
  (add `self.OnPartHoveredBegin` (`|CreateDelegate` :!event `HandleOnAxisHoveredBegin`))
  (add `self.OnPartHoveredEnd` (`|CreateDelegate` :!event `HandleOnAxisHoveredEnd`)))

(fn `DeselectAxis`
  (params (Axis :type "/SZDebugger/BP/Enum/E_SelectedAxis Enum" :default "NewEnumerator3"))
  (`PrimitiveComponent.SetMaterial` (`self.EAxisToAxisSM` Axis) 0 (`self.EAxisToAxisDefaultMat` Axis))
  (set `self.SelectedAxis` "NewEnumerator3"))

(fn `DeselectSelectedAxis`
  (if (`|EnumInequality` (`self.SelectedAxis`) "NewEnumerator3")
    (`self.DeselectAxis` (`self.SelectedAxis`))))

(fn `EAxisToAxisDefaultMat`
  (params (Axis :type "/SZDebugger/BP/Enum/E_SelectedAxis Enum" :default "NewEnumerator3"))
  (returns (ReturnValue :type "MaterialInterface Object Reference"))
  (return (select `/SZDebugger/BP/Enum/E_SelectedAxis` Axis :`NewEnumerator0` "/SZDebugger/Material/MI_Axis_X.MI_Axis_X" :`NewEnumerator1` "/SZDebugger/Material/MI_Axis_Y.MI_Axis_Y" :`NewEnumerator2` "/SZDebugger/Material/MI_Axis_Z.MI_Axis_Z" :`NewEnumerator4` "/SZDebugger/Material/MI_Axis_All.MI_Axis_All" :!type "MaterialInterface Object Reference")))

(fn `EAxisToAxisSM`
  (params (Axis :type "/SZDebugger/BP/Enum/E_SelectedAxis Enum" :default "NewEnumerator0"))
  (returns (ReturnValue :type "PrimitiveComponent Object Reference"))
  (return (select `/SZDebugger/BP/Enum/E_SelectedAxis` Axis :`NewEnumerator0` (`self.X`) :`NewEnumerator1` (`self.Y`) :`NewEnumerator2` (`self.Z`) :`NewEnumerator4` (`self.All`))))

(fn `GetWorldAxisVecFromEAxis`
  (params (Axis :type "/SZDebugger/BP/Enum/E_SelectedAxis Enum" :default "NewEnumerator3"))
  (returns (ReturnValue :type "Vector Structure"))
  (if (`|EnumInequality` Axis "NewEnumerator3")
    (return (`SceneComponent.GetForwardVector` (`self.EAxisToAxisSM` Axis)))
    (else
      (return (-1.0 -1.0 -1.0)))))

(fn `GetWorldAxisVecFromSelectedAxis`
  (returns (ReturnValue :type "Vector Structure"))
  (return (`self.GetWorldAxisVecFromEAxis` (`self.SelectedAxis`))))

(fn `HandleOnAxisHoveredBegin`
  (params (Axis :type "/SZDebugger/BP/Enum/E_SelectedAxis Enum" :default "NewEnumerator3"))
  (if (not (`self.SelectionLock`))
    (`self.DeselectSelectedAxis`)
    (`self.SelectAxis` Axis)))

(fn `HandleOnAxisHoveredEnd`
  (if (not (`self.SelectionLock`))
    (`self.DeselectSelectedAxis`)))

(fn `IsAxisSelected`
  (returns (ReturnValue :type Boolean))
  (return (`|EnumInequality` (`self.SelectedAxis`) "NewEnumerator3")))

(fn `LockSelection`
  (set `self.SelectionLock` true))

(fn `SelectAxis`
  (params (Axis :type "/SZDebugger/BP/Enum/E_SelectedAxis Enum" :default "NewEnumerator0"))
  (bind _output_get (set `self.SelectedAxis` Axis))
  (`PrimitiveComponent.SetMaterial` (`self.EAxisToAxisSM` _output_get) 0 (`self.SelectedAxisMat`)))

(fn `SetAbsoluteRotation`
  (params (bNewAbsoluteRotation :type Boolean))
  (`SceneComponent.SetAbsolute` (`self.Parent`) false bNewAbsoluteRotation true)
  (set `self.UseAbsoluteRot` bNewAbsoluteRotation))

(fn `SetAxesRotation`
  (params (X :type "Rotator Structure") (Y :type "Rotator Structure") (Z :type "Rotator Structure") (WorldRot :type Boolean))
  (if WorldRot
    (`SceneComponent.K2_SetWorldRotation` (`self.X`) X false false)
    (`SceneComponent.K2_SetWorldRotation` (`self.Y`) Y false false)
    (`SceneComponent.K2_SetWorldRotation` (`self.Z`) Z false false)
    (else
      (`SceneComponent.K2_SetRelativeRotation` (`self.X`) X false false)
      (`SceneComponent.K2_SetRelativeRotation` (`self.Y`) Y false false)
      (`SceneComponent.K2_SetRelativeRotation` (`self.Z`) Z false false))))

(fn `SetAxesScale`
  (params (NewScale :type "Vector Structure"))
  (`SceneComponent.SetWorldScale3D` (`self.Parent`) NewScale))

(fn `SetAxesType`
  (params (NewAxisType :type "/SZDebugger/BP/Enum/E_AxisType Enum" :default "NewEnumerator0"))
  (bind _returnvalue (select `/SZDebugger/BP/Enum/E_AxisType` (`self.Axis Type`) :`NewEnumerator0` "/SZDebugger/Mesh/ArrowAxis.ArrowAxis" :`NewEnumerator1` "/SZDebugger/Mesh/RotatorAxis.RotatorAxis" :`NewEnumerator2` "/SZDebugger/Mesh/ScaleAxis.ScaleAxis" :!type "StaticMesh Object Reference"))
  (bind _output_get (set `self.Axis Type` NewAxisType))
  (`SceneComponent.SetHiddenInGame` (`self.All`) (`|EnumEquality` _output_get "NewEnumerator1") false)
  (`StaticMeshComponent.SetStaticMesh` (`self.X`) _returnvalue)
  (`StaticMeshComponent.SetStaticMesh` (`self.Y`) _returnvalue)
  (`StaticMeshComponent.SetStaticMesh` (`self.Z`) _returnvalue)
  (if (`|EnumEquality` (`self.Axis Type`) "NewEnumerator1")
    (`self.SetAxesRotation` (struct :`Yaw` 90.0) (struct) (struct :`Roll` 90.0))
    (else
      (`self.SetAxesRotation` (struct) (struct :`Yaw` 90.0) (struct :`Pitch` 90.0)))))

(fn `UnlockSelection`
  (set `self.SelectionLock` false)
  (`self.DeselectSelectedAxis`))

(fn `UserConstructionScript`)